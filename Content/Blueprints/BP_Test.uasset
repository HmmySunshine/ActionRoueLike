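; BP_Test is a test Blueprint that counts projectile hits on its Sphere component and shows the score on a TextRender.
; On each hit it gathers all Projectile actors, but the loop body is empty, so only the leftover array element is compared with OtherActor.
; A match increments Score and updates the text; otherwise it prints a debug string.
; A separate Hehe function only prints a placeholder string.
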(event `self.ReceiveBeginPlay`)

(event `self.Sphere.OnComponentHit`
  (params (HitComponent :type "PrimitiveComponent Object Reference") (OtherActor :type "Actor Object Reference") (OtherComp :type "PrimitiveComponent Object Reference") (NormalImpulse :type "Vector Structure") (Hit :type "HitResult Structure (by ref)"))
  (bind _outactors (`GameplayStatics.GetAllActorsOfClass` "/Game/Blueprints/Projectile.Projectile_C"))
  (for _array_element _outactors
    _)
  (if (== OtherActor _array_element)
    (bind _output_get (set `self.score` (+ (`self.score`) 1)))
    (`TextRenderComponent.K2_SetText` (`self.TextRender`) (`KismetTextLibrary.Conv_StringToText` (`KismetTextLibrary.Conv_TextToString` (`KismetTextLibrary.Conv_Int64ToText` _output_get))))
    (else
      (`KismetSystemLibrary.PrintString` "Hello"))))

(fn `hehe`
  (`KismetSystemLibrary.PrintString` "jilegggg"))

(fn `UserConstructionScript`)